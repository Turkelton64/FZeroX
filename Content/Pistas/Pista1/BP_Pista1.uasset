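; BP_Pista1 is a track Blueprint that builds its mesh procedurally along the RoadTrack spline.
; The construction script divides the spline length by Distancia and adds a spline mesh component using StaticMesh for each segment.
; Each segment takes its local endpoints and directions from the spline, with directions scaled by Tangente to form tangents.
; The event graph holds only disabled default events, so it adds no runtime logic.
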(fn `UserConstructionScript`
  (bind _roadtrack (`self.RoadTrack`))
  (bind _distancia (`self.Distancia`))
  (for _index (range (+ (`.ReturnValue` (`KismetMathLibrary.FMod` (`SplineComponent.GetSplineLength` (`self.RoadTrack`)) (`self.Distancia`))) 1))
    (bind _returnvalue (`AddComponent|NODE_AddSplineMeshComponent-0`))
    (`StaticMeshComponent.SetStaticMesh` _returnvalue (`self.Static Mesh`))
    (bind _returnvalue_2 (* _index _distancia))
    (bind _returnvalue_3 (+ _returnvalue_2 _distancia))
    (`SplineMeshComponent.SetStartAndEnd` _returnvalue (`SplineComponent.GetLocationAtDistanceAlongSpline` _roadtrack _returnvalue_2 "Local") (* (`SplineComponent.GetDirectionAtDistanceAlongSpline` _roadtrack _returnvalue_2 "Local") (`self.Tangente`)) (`SplineComponent.GetLocationAtDistanceAlongSpline` _roadtrack _returnvalue_3 "Local") (* (`SplineComponent.GetDirectionAtDistanceAlongSpline` _roadtrack _returnvalue_3 "Local") (`self.Tangente`)) true)))
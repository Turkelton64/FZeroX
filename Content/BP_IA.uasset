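; AI racer Blueprint that moves a vehicle along the spline of a referenced track (PistaRef).
; On BeginPlay it places Base on the spline, then a looping Correr timer turns it along the spline and adds forward velocity impulses, advancing a distance counter independently of actual position.
; Two alternative movers exist, not called here: MoverNave's timeline interpolation, and Prueba's timer-driven IniciarCarrera, which steps the actor until the spline ends.
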(event `self.ReceiveBeginPlay`
  (`SceneComponent.K2_SetWorldLocationAndRotation` :`self` (`self.Base`) :`NewLocation` (`SplineComponent.GetLocationAtDistanceAlongSpline` (`/Game/BP_SpliteLineIA.UsefullSpline` (`self.PistaRef`)) (`self.DistanciaActual`) "World"))
  (`KismetSystemLibrary.K2_SetTimer` null "Correr" 0.1 true))

(event `MoverNave`
  (bind _movimiento_coche (`self.Movimiento Coche`))
  (bind _usefullspline (`/Game/BP_SpliteLineIA.UsefullSpline` (`self.PistaRef`)))
  (bind _returnvalue (`KismetMathLibrary.Lerp` 0.0 (`SplineComponent.GetSplineLength` _usefullspline) (`self.Alpha`)))
  (`TimelineComponent.SetPlayRate` _movimiento_coche (/ 1.0 (`self.Duration`)))
  (`TimelineComponent.SetNewTime` _movimiento_coche (`self.DireccionInicioNave`))
  (bind (_direction _alpha) (`Timeline|Movimiento Coche`)
    (:`Update`
      (set `self.Alpha` _alpha)
      (`self.K2_SetActorLocationAndRotation` (`SplineComponent.GetLocationAtDistanceAlongSpline` _usefullspline _returnvalue "World") (`SplineComponent.GetRotationAtDistanceAlongSpline` _usefullspline _returnvalue "World")))))

(event `Prueba`
  (set `self.DistanciaDeCircuito` (`SplineComponent.GetSplineLength` (`/Game/BP_SpliteLineIA.UsefullSpline` (`self.PistaRef`))))
  (`KismetSystemLibrary.K2_SetTimer` null "IniciarCarrera" 0.05 true))

(fn `Correr`
  (bind _base (`self.Base`))
  (`SceneComponent.K2_SetWorldRotation` (`self.Base`) (`SplineComponent.GetRotationAtDistanceAlongSpline` (`/Game/BP_SpliteLineIA.UsefullSpline` (`self.PistaRef`)) (+ (`self.DistanciaActual`) 1.0) "World") false false)
  (`PrimitiveComponent.AddImpulse` _base (* (`SceneComponent.GetForwardVector` _base) 2.0) "None" true)
  (set `self.DistanciaActual` (+ (`self.DistanciaActual`) 1.0)))

(fn `IniciarCarrera`
  (bind _distanciaactual (`self.DistanciaActual`))
  (bind _usefullspline (`/Game/BP_SpliteLineIA.UsefullSpline` (`self.PistaRef`)))
  (set `self.DistanciaActual` (+ (`self.DistanciaActual`) 100.0))
  (if (<= (`self.DistanciaActual`) (`self.DistanciaDeCircuito`))
    (`self.K2_SetActorLocationAndRotation` (`SplineComponent.GetLocationAtDistanceAlongSpline` _usefullspline _distanciaactual "World") (`SplineComponent.GetRotationAtDistanceAlongSpline` _usefullspline _distanciaactual "World"))
    (`KismetSystemLibrary.PrintString` "Hello")
    (else
      (`KismetSystemLibrary.K2_ClearTimer` null "IniciarCarrera")
      (`KismetSystemLibrary.PrintString` "2"))))

(fn `UserConstructionScript`)
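; BP_Nave is a ship actor moved by physics impulses on its Cuerpo component.
; On BeginPlay it enables input from player controller 0 and sets that controller's view target to the player character.
; Three functions, not called within this Blueprint, accelerate or push it left or right with fixed world-axis velocity-change impulses and print debug text.
; The turn functions apply no rotation, and the accelerate function's extra AddForce is zero.
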(event `self.ReceiveBeginPlay`
  (`self.EnableInput` (`GameplayStatics.GetPlayerController` 0))
  (`PlayerController.SetViewTargetWithBlend` (`GameplayStatics.GetPlayerController` 0) (`GameplayStatics.GetPlayerCharacter` 0) 0.0 "VTBlend_Linear" 3.0 false))

(fn `Fctn_Acelerar`
  (`PrimitiveComponent.AddImpulse` (`self.Cuerpo`) (100.0 0.0 0.0) "None" true)
  (`KismetSystemLibrary.PrintString` "Acelerar")
  (`PrimitiveComponent.AddForce` (`self.Cuerpo`) (0.0 0.0 0.0) "None" false))

(fn `Fctn_Girar_Derecha`
  (`PrimitiveComponent.AddImpulse` (`self.Cuerpo`) (0.0 100.0 0.0) "None" true)
  (`KismetSystemLibrary.PrintString` "Derecha"))

(fn `Fctn_Girar_Izquierda`
  (`PrimitiveComponent.AddImpulse` (`self.Cuerpo`) (0.0 -100.0 0.0) "None" true)
  (`KismetSystemLibrary.PrintString` "Izquierda"))

(fn `UserConstructionScript`)
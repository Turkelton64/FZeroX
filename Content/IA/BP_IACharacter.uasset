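; AI character for a ship (Nave) that tilts to follow the landscape's slope.
; Each tick, ComprobarSuelo traces from front and rear probe components, continuing only on Landscape hits.
; When the two distances differ beyond a small tolerance, it nudges capsule pitch a fixed step per frame, without delta-time scaling.
; BeginPlay applies movement limits and stores the AI controller; hits on Nave decrement Energia, which nothing here reads.
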(event `self.ReceiveTick`
  (params (DeltaSeconds :type "Float (single-precision)"))
  (`self.ComprobarSuelo`))

(event `self.ReceiveBeginPlay`
  (bind _charactermovement (`self.CharacterMovement`))
  (set `CharacterMovementComponent.MaxWalkSpeed` (`self.MaxVelocity`) _charactermovement)
  (set `CharacterMovementComponent.MaxAcceleration` (`self.MaxAceleration`) _charactermovement)
  (set `self.ControlledPawn` (`AIBlueprintHelperLibrary.GetAIController` self)))

(event `self.Nave.OnComponentHit`
  (params (HitComponent :type "PrimitiveComponent Object Reference") (OtherActor :type "Actor Object Reference") (OtherComp :type "PrimitiveComponent Object Reference") (NormalImpulse :type "Vector Structure") (Hit :type "HitResult Structure (by ref)"))
  (set `self.Energia` (- (`self.Energia`) 1.0)))

(fn `ComprobarSuelo`
  (locals (DistanciaDelMorro :type "Float (double-precision)" :default 0.0) (DistanciaDelCulo :type "Float (double-precision)"))
  (bind _distanciadelantera (`self.DistanciaDelantera`))
  (bind _distanciatrasera (`self.DistanciaTrasera`))
  (bind _capsulecomponent (`self.CapsuleComponent`))
  (bind _capsulecomponent_2 (`self.CapsuleComponent`))
  (bind _returnvalue (`SceneComponent.K2_GetComponentLocation` _distanciatrasera))
  (bind _returnvalue_2 (`SceneComponent.K2_GetComponentLocation` _distanciadelantera))
  (bind (_outhit _returnvalue_3) (`KismetSystemLibrary.LineTraceSingle` _returnvalue_2 (+ _returnvalue_2 (* (`KismetMathLibrary.GetForwardVector` (`SceneComponent.K2_GetComponentRotation` _distanciadelantera)) 1500.0)) "TraceTypeQuery1"))
  (if _returnvalue_3
    (bind (_bblockinghit _binitialoverlap _time _distance _location _impactpoint _normal _impactnormal _physmat _hitactor) (`GameplayStatics.BreakHitResult` _outhit))
    (cast `Landscape` _hitactor)
    (set `local.DistanciaDelMorro` _distance)
    (bind (_outhit_2 _returnvalue_4) (`KismetSystemLibrary.LineTraceSingle` _returnvalue (+ _returnvalue (* (`KismetMathLibrary.GetForwardVector` (`SceneComponent.K2_GetComponentRotation` _distanciatrasera)) 1500.0)) "TraceTypeQuery1"))
    (if _returnvalue_4
      (bind (_bblockinghit_2 _binitialoverlap_2 _time_2 _distance_2 _location_2 _impactpoint_2 _normal_2 _impactnormal_2 _physmat_2 _hitactor_2) (`GameplayStatics.BreakHitResult` _outhit_2))
      (cast `Landscape` _hitactor_2)
      (bind _output_get (set `local.DistanciaDelCulo` _distance_2))
      (if (`KismetMathLibrary.NearlyEqual_FloatFloat` _output_get (`local.DistanciaDelMorro`) 2.0)
        _
        (elif (< (`local.DistanciaDelMorro`) (`local.DistanciaDelCulo`))
          (`SceneComponent.K2_SetWorldRotation` _capsulecomponent_2 (`KismetMathLibrary.MakeRotator` (.roll (`SceneComponent.K2_GetComponentRotation` _capsulecomponent_2)) (+ (.pitch (`SceneComponent.K2_GetComponentRotation` _capsulecomponent_2)) 1.0) (.yaw (`SceneComponent.K2_GetComponentRotation` _capsulecomponent_2))) false false)
          (else
            (`SceneComponent.K2_SetWorldRotation` _capsulecomponent (`KismetMathLibrary.MakeRotator` (.roll (`SceneComponent.K2_GetComponentRotation` _capsulecomponent)) (- (.pitch (`SceneComponent.K2_GetComponentRotation` _capsulecomponent)) 1.0) (.yaw (`SceneComponent.K2_GetComponentRotation` _capsulecomponent))) false false)))))))

(fn `UserConstructionScript`)
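; AI race character that navigates to the first target point of a BP_IATracks actor and tracks its closest spline key each tick.
; Overlapping the third found TriggerBox starts a timeline that carries it along the track's first spline, then navigation to that point resumes.
; Paired-trace pitch/roll surface alignment, waypoint cycling and energy-depletion explosions are written, but their timers and energy check are never run.
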(event `self.ReceiveTick`
  (params (DeltaSeconds :type "Float (single-precision)"))
  (set `self.Distancia` (`SplineComponent.FindInputKeyClosestToWorldLocation` (`/Game/IA/BP_IASpline.Camino` (`self.Spline`)) (`SceneComponent.K2_GetComponentLocation` (`self.STMesh`)))))

(event `self.ReceiveBeginPlay`
  (`self.IniciarCarrera`))

(event `IniciarCarrera`
  (bind _outactors (`GameplayStatics.GetAllActorsOfClass` "/Game/IA/BP_IATracks.BP_IATracks_C"))
  (bind _output_get (set `self.IATracks` (`|GetArrayItem` _outactors)))
  (`AIController.MoveToLocation` (`AIBlueprintHelperLibrary.GetAIController` self) (`SceneComponent.K2_GetComponentLocation` (`TargetPoint.SpriteComponent` (`|GetArrayItem` (`/Game/IA/BP_IATracks.TargetPoints` _output_get)))) -1.0 true true true false null false)
  (bind _outactors_2 (`GameplayStatics.GetAllActorsOfClass` "/Script/Engine.TriggerBox"))
  (add `self.OnActorBeginOverlap` (`|GetArrayItem` _outactors_2 2) (delegate `IniciarVuelo`)))

(event `IniciarVuelo` :!signature `self.OnActorBeginOverlap`
  (params (OverlappedActor :type "Actor Object Reference") (OtherActor :type "Actor Object Reference"))
  (bind _asbp_aicharacter (cast `/Game/IA/BP_AICharacter` OtherActor))
  (`self.EventoAnimacionVuelo` _asbp_aicharacter _asbp_aicharacter))

(event `EventoAnimacionVuelo`
  (params (AICharacter :type "/Game/IA/BP_AICharacter Object Reference"))
  (bind _camino (`/Game/IA/BP_IASpline.Camino` (`|GetArrayItem` (`/Game/IA/BP_IATracks.Splines` (`self.IATracks`)))))
  (bind _returnvalue (`KismetMathLibrary.Lerp` 0.0 (`SplineComponent.GetSplineLength` _camino) (`self.Alpha`)))
  (bind (_direction _alpha) (`Timeline|AnimacionVuelo` :!via `PlayFromStart`)
    (:`Update`
      (set `self.Alpha` _alpha)
      (`self.K2_SetActorLocationAndRotation` AICharacter (`SplineComponent.GetLocationAtDistanceAlongSpline` _camino _returnvalue "World") (`SplineComponent.GetRotationAtDistanceAlongSpline` _camino _returnvalue "World") false false))
    (:`Finished`
      (`AIController.MoveToLocation` (`AIBlueprintHelperLibrary.GetAIController` AICharacter) (`SceneComponent.K2_GetComponentLocation` (`TargetPoint.SpriteComponent` (`|GetArrayItem` (`/Game/IA/BP_IATracks.TargetPoints` (`self.IATracks`))))) -1.0 true true true false null false))))

(event `self.STMesh.OnComponentHit`
  (params (HitComponent :type "PrimitiveComponent Object Reference") (OtherActor :type "Actor Object Reference") (OtherComp :type "PrimitiveComponent Object Reference") (NormalImpulse :type "Vector Structure") (Hit :type "HitResult Structure (by ref)")))

(event `AnimacionSinEnergia`
  (`Timeline|ASinEnergia` :!via `PlayFromStart`
    (:`Update`
      (`|SpawnActorFromClass` "/Game/StarterContent/Blueprints/Blueprint_Effect_Explosion.Blueprint_Effect_Explosion_C" (`SceneComponent.K2_GetComponentToWorld` (`self.STMesh`)) "Undefined" "OverrideRootScale" null null))
    (:`Finished`
      (`KismetSystemLibrary.PrintString` "BOOOOOOOOOOOOOOOOM!!!!"))))

(fn `ActualizarMeta`
  (locals (NewLocalVar_0 :type "EPathFollowingRequestResult Enum" :default "Failed"))
  (bind _targetpoints (`/Game/IA/BP_IATracks.TargetPoints` (`self.IATracks`)))
  (`KismetSystemLibrary.PrintString` (`KismetStringLibrary.Conv_IntToString` (`self.GoalIndex`)))
  (if (`KismetMathLibrary.NearlyEqual_FloatFloat` (- (`KismetMathLibrary.VSize` (`SceneComponent.K2_GetComponentLocation` (`self.CapsuleComponent`))) (`KismetMathLibrary.VSize` (`SceneComponent.K2_GetComponentLocation` (`TargetPoint.SpriteComponent` (`|GetArrayItem` (`/Game/IA/BP_IATracks.TargetPoints` (`self.IATracks`)) (`self.GoalIndex`)))))) 0.0 20.0)
    (bind _output_get (set `self.GoalIndex` (+ (`self.GoalIndex`) 1)))
    (if (== _output_get (`KismetArrayLibrary.Array_Length` _targetpoints))
      (set `self.GoalIndex` 0))
    (`AIController.MoveToLocation` (`AIBlueprintHelperLibrary.GetAIController` self) (`SceneComponent.K2_GetComponentLocation` (`TargetPoint.SpriteComponent` (`|GetArrayItem` _targetpoints (`self.GoalIndex`)))) -1.0 true true true false null false)))

(fn `DistanciaHorizontal`
  (locals (DistanciaLDerecha :type "Float (double-precision)") (DistanciaLIzquierda :type "Float (double-precision)") (Base :type "Float (double-precision)") (Altura :type "Float (double-precision)") (TAN :type "Float (double-precision)") (ATAN :type "Float (double-precision)"))
  (bind _capsulecomponent (`self.CapsuleComponent`))
  (bind _distanciaderecha (`self.DistanciaDerecha`))
  (bind _distanciaizquierda (`self.DistanciaIzquierda`))
  (bind _returnvalue (`SceneComponent.K2_GetComponentLocation` _distanciaderecha))
  (bind _returnvalue_2 (`SceneComponent.K2_GetComponentLocation` _distanciaizquierda))
  (bind (_outhit _returnvalue_3) (`KismetSystemLibrary.LineTraceSingle` :`Start` _returnvalue :`End` (+ _returnvalue (* (`KismetMathLibrary.GetForwardVector` (`SceneComponent.K2_GetComponentRotation` _distanciaderecha)) 150.0)) :`TraceChannel` "TraceTypeQuery1" :`DrawDebugType` "ForOneFrame"))
  (if _returnvalue_3
    (set `local.DistanciaLDerecha` (`.Distance` (`GameplayStatics.BreakHitResult` _outhit)))
    (bind (_outhit_2 _returnvalue_4) (`KismetSystemLibrary.LineTraceSingle` :`Start` _returnvalue_2 :`End` (+ _returnvalue_2 (* (`KismetMathLibrary.GetForwardVector` (`SceneComponent.K2_GetComponentRotation` _distanciaizquierda)) 150.0)) :`TraceChannel` "TraceTypeQuery1" :`DrawDebugType` "ForOneFrame"))
    (if _returnvalue_4
      (set `local.DistanciaLIzquierda` (`.Distance` (`GameplayStatics.BreakHitResult` _outhit_2)))
      (if (not (`KismetMathLibrary.NearlyEqual_FloatFloat` (`local.DistanciaLIzquierda`) (`local.DistanciaLDerecha`) 0.1))
        (set `local.Base` (`KismetMathLibrary.VSize` (- (`SceneComponent.K2_GetComponentLocation` (`self.DistanciaDerecha`)) (`SceneComponent.K2_GetComponentLocation` (`self.DistanciaIzquierda`)))))
        (if (> (`local.DistanciaLDerecha`) (`local.DistanciaLIzquierda`))
          (bind _output_get (set `local.Altura` (- (`local.DistanciaLIzquierda`) (`local.DistanciaLDerecha`))))
          (bind _output_get_2 (set `local.TAN` (/ _output_get (`local.Base`))))
          (set `local.ATAN` (* (`KismetMathLibrary.DegAtan` _output_get_2) -1.0))
          (else
            (bind _output_get_3 (set `local.Altura` (- (`local.DistanciaLDerecha`) (`local.DistanciaLIzquierda`))))
            (bind _output_get_4 (set `local.TAN` (/ _output_get_3 (`local.Base`))))
            (set `local.ATAN` (`KismetMathLibrary.DegAtan` _output_get_4))))
        (`SceneComponent.K2_SetWorldRotation` _capsulecomponent (`KismetMathLibrary.MakeRotator` (+ (.roll (`SceneComponent.K2_GetComponentRotation` _capsulecomponent)) (`local.ATAN`)) (.pitch (`SceneComponent.K2_GetComponentRotation` _capsulecomponent)) (.yaw (`SceneComponent.K2_GetComponentRotation` _capsulecomponent))) false false)))))

(fn `DistanciaVertical`
  (locals (DistanciaDelCulo :type "Float (double-precision)") (DistanciaDelMorro :type "Float (double-precision)") (Base :type "Float (double-precision)") (Altura :type "Float (double-precision)") (TAN :type "Float (double-precision)") (ATAN :type "Float (double-precision)"))
  (bind _distanciadelantera (`self.DistanciaDelantera`))
  (bind _distanciatrasera (`self.DistanciaTrasera`))
  (bind _capsulecomponent (`self.CapsuleComponent`))
  (bind _returnvalue (`SceneComponent.K2_GetComponentLocation` _distanciadelantera))
  (bind _returnvalue_2 (`SceneComponent.K2_GetComponentLocation` _distanciatrasera))
  (bind (_outhit _returnvalue_3) (`KismetSystemLibrary.LineTraceSingle` :`Start` _returnvalue :`End` (+ _returnvalue (* (`KismetMathLibrary.GetForwardVector` (`SceneComponent.K2_GetComponentRotation` _distanciadelantera)) 150.0)) :`TraceChannel` "TraceTypeQuery1" :`DrawDebugType` "ForOneFrame"))
  (if _returnvalue_3
    (set `local.DistanciaDelMorro` (`.Distance` (`GameplayStatics.BreakHitResult` _outhit)))
    (bind (_outhit_2 _returnvalue_4) (`KismetSystemLibrary.LineTraceSingle` :`Start` _returnvalue_2 :`End` (+ _returnvalue_2 (* (`KismetMathLibrary.GetForwardVector` (`SceneComponent.K2_GetComponentRotation` _distanciatrasera)) 150.0)) :`TraceChannel` "TraceTypeQuery1" :`DrawDebugType` "ForOneFrame"))
    (if _returnvalue_4
      (set `local.DistanciaDelCulo` (`.Distance` (`GameplayStatics.BreakHitResult` _outhit_2)))
      (if (not (`KismetMathLibrary.NearlyEqual_FloatFloat` (`local.DistanciaDelCulo`) (`local.DistanciaDelMorro`) 0.1))
        (set `local.Base` (`KismetMathLibrary.VSize` (- (`SceneComponent.K2_GetComponentLocation` (`self.DistanciaDelantera`)) (`SceneComponent.K2_GetComponentLocation` (`self.DistanciaTrasera`)))))
        (if (> (`local.DistanciaDelMorro`) (`local.DistanciaDelCulo`))
          (bind _output_get (set `local.Altura` (- (`local.DistanciaDelMorro`) (`local.DistanciaDelCulo`))))
          (bind _output_get_2 (set `local.TAN` (/ _output_get (`local.Base`))))
          (set `local.ATAN` (* (`KismetMathLibrary.DegAtan` _output_get_2) -1.0))
          (else
            (bind _output_get_3 (set `local.Altura` (- (`local.DistanciaDelCulo`) (`local.DistanciaDelMorro`))))
            (bind _output_get_4 (set `local.TAN` (/ _output_get_3 (`local.Base`))))
            (set `local.ATAN` (`KismetMathLibrary.DegAtan` _output_get_4))))
        (`SceneComponent.K2_SetWorldRotation` _capsulecomponent (`KismetMathLibrary.MakeRotator` (.roll (`SceneComponent.K2_GetComponentRotation` _capsulecomponent)) (+ (.pitch (`SceneComponent.K2_GetComponentRotation` _capsulecomponent)) (`local.ATAN`)) (.yaw (`SceneComponent.K2_GetComponentRotation` _capsulecomponent))) false false)))))

(fn `UserConstructionScript`)
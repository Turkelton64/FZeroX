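; Race-start sign actor whose robot "RoboGo" shows a 3-2-1-GO countdown.
; IniciarCuentaAtras plays the countdown sound and runs a self-calling event that swaps timer materials each second, flashing both robot faces' mouths open and closed.
; IniciarAnimacion uses a timeline to slide the structure along the Ruta spline.
; Two seconds after BeginPlay, the root moves to the first BP_Nave's forward vector, used directly as a world location.
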(event `self.ReceiveBeginPlay`
  (`KismetSystemLibrary.Delay` 2.0)
  (bind _outactors (`GameplayStatics.GetAllActorsOfClass` "/Game/BP_Nave.BP_Nave_C"))
  (`SceneComponent.K2_SetWorldLocation` (`self.DefaultSceneRoot`) (`SceneComponent.GetForwardVector` (`/Game/BP_Nave.Nave` (`|GetArrayItem` _outactors))) false false))

(event `IniciarAnimacion`
  (bind _ruta (`self.Ruta`))
  (bind (_direction _newtrack_0) (`Timeline|Timeline_0`)
    (:`Update`
      (`SceneComponent.K2_SetWorldLocation` (`self.Structura`) (`SplineComponent.GetLocationAtDistanceAlongSpline` _ruta (`KismetMathLibrary.Lerp` 0.0 (`SplineComponent.GetSplineLength` _ruta) _newtrack_0) "World") false false))))

(event `IniciarCuentaAtras`
  (`GameplayStatics.SpawnSound2D` "/Game/Interfaces/Sonidos/321GoTheme.321GoTheme" 1.0 1.0 0.0 null)
  (`self.AnimacionRoboGo`))

(event `AnimacionRoboGo`
  (if (== (`self.TemporizadorRoboGo`) 0)
    (`PrimitiveComponent.SetMaterial` (`self.RoboGoTemporizador`) 0 "/Game/Interfaces/Materiales/MaterialRoboGo_3.MaterialRoboGo_3")
    (`self.RoboGoAnimacionAbrirBoca` :!label _label)
    (`KismetSystemLibrary.Delay` 0.2)
    (`self.RoboGoAnimacionCerrarBoca`)
    (`KismetSystemLibrary.Delay` 0.8)
    (set `self.TemporizadorRoboGo` (+ (`self.TemporizadorRoboGo`) 1))
    (`self.AnimacionRoboGo`)
    (elif (== (`self.TemporizadorRoboGo`) 1)
      (`PrimitiveComponent.SetMaterial` (`self.RoboGoTemporizador`) 0 "/Game/Interfaces/Materiales/MaterialRoboGo_2.MaterialRoboGo_2")
      (goto _label)
      (elif (== (`self.TemporizadorRoboGo`) 2)
        (`PrimitiveComponent.SetMaterial` (`self.RoboGoTemporizador`) 0 "/Game/Interfaces/Materiales/MaterialRoboGo_1.MaterialRoboGo_1")
        (goto _label)
        (else
          (`PrimitiveComponent.SetMaterial` (`self.RoboGoTemporizador`) 0 "/Game/Interfaces/Materiales/MaterialRoboGo_GO.MaterialRoboGo_GO"))))))

(fn `RoboGoAnimacionAbrirBoca`
  (`PrimitiveComponent.SetMaterial` (`self.RoboGoDer`) 0 "/Game/Interfaces/Materiales/MaterialRoboGo_State2.MaterialRoboGo_State2")
  (`PrimitiveComponent.SetMaterial` (`self.RoboGoIzq`) 0 "/Game/Interfaces/Materiales/MaterialRoboGo_State2.MaterialRoboGo_State2"))

(fn `RoboGoAnimacionCerrarBoca`
  (`PrimitiveComponent.SetMaterial` (`self.RoboGoDer`) 0 "/Game/Interfaces/Materiales/MaterialRoboGo_State1.MaterialRoboGo_State1")
  (`PrimitiveComponent.SetMaterial` (`self.RoboGoIzq`) 0 "/Game/Interfaces/Materiales/MaterialRoboGo_State1.MaterialRoboGo_State1"))

(fn `UserConstructionScript`)
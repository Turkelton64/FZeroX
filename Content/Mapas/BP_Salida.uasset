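; BP_Salida is the start/finish line of an F-Zero-style race, counting laps for the player's BP_Nave.
; Two level trigger boxes set checkpoint flags, and crossing its Box with both set increments the lap on the ship's interface.
; Lap three outside Practice plays the finish animation and overwrites the map's GameInstance best time with the race time.
; Other laps re-arm after a delay, checking lap time and resetting checkpoints outside GP.
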(event `self.ReceiveBeginPlay`
  (bind _asfzero_game_instance (cast `/Game/Interfaces/FZero_GameInstance` (`GameplayStatics.GetGameInstance`)))
  (set `self.GameInstance` _asfzero_game_instance)
  (add `self.OnActorBeginOverlap` (`self.TriggerBoxInicial`) (delegate `CheckPoint1`))
  (add `self.OnActorBeginOverlap` (`self.TriggerBoxFinal`) (delegate `CheckPoint2`)))

(event `CheckPoint1` :!signature `self.OnActorBeginOverlap`
  (params (OverlappedActor :type "Actor Object Reference") (OtherActor :type "Actor Object Reference"))
  (set `self.CP_1` true)
  (set `self.CP_2` false)
  (`KismetSystemLibrary.PrintString` "1"))

(event `CheckPoint2` :!signature `self.OnActorBeginOverlap`
  (params (OverlappedActor :type "Actor Object Reference") (OtherActor :type "Actor Object Reference"))
  (set `self.CP_2` true)
  (`KismetSystemLibrary.PrintString` "2"))

(event `self.Box.OnComponentBeginOverlap`
  (params (OverlappedComponent :type "PrimitiveComponent Object Reference") (OtherActor :type "Actor Object Reference") (OtherComp :type "PrimitiveComponent Object Reference") (OtherBodyIndex :type Integer) (bFromSweep :type Boolean) (SweepResult :type "HitResult Structure (by ref)"))
  (bind _gameinstance (`self.GameInstance`))
  (bind _mapaactual (`/Game/Interfaces/FZero_GameInstance.MapaActual` _gameinstance))
  (bind (_mejorestiemposporpista _mejortiempoenpista) (break `/Game/Interfaces/EstructurasDeDatos/BP_Estructura_DatosGuardadosJugador` (`/Game/Interfaces/FZero_GameInstance.DatosJugador` _gameinstance)))
  (if (and (== (`GameplayStatics.GetPlayerPawn` 0) OtherActor) (`self.SWEscuchar`))
    (set `self.SWEscuchar` false)
    (if (and (`self.CP_1`) (`self.CP_2`))
      (bind _asbp_nave (cast `/Game/BP_Nave` OtherActor))
      (bind _interface (`/Game/BP_Nave.Interface` _asbp_nave))
      (bind _output_get (set `/Game/Interfaces/BP_GUI_Carrera.LapActual` (+ (`/Game/Interfaces/BP_GUI_Carrera.LapActual` _interface) 1) _interface))
      (if (and (== _output_get 3) (`KismetStringLibrary.NotEqual_StrStr` (`/Game/Interfaces/FZero_GameInstance.ModoJuego` (`self.GameInstance`)) "Practice"))
        (`UserWidget.PlayAnimation` _interface (`/Game/Interfaces/BP_GUI_Carrera.AnimacionFinish` _interface) 0.0 1 "Forward" 1.0 false)
        (if (== (`/Game/Interfaces/BP_GUI_Carrera.BestTime` _interface) 0)
          (`Widget.SetVisibility` (`/Game/Interfaces/BP_GUI_Carrera.TX_BESTTIME` _interface) "Visible")
          (else
            (`BlueprintMapLibrary.Map_Remove` _mejortiempoenpista _mapaactual)))
        (bind _tiempodecarrera (`/Game/Interfaces/BP_GUI_Carrera.TiempoDeCarrera` _interface))
        (`BlueprintMapLibrary.Map_Add` _mejortiempoenpista _mapaactual (`KismetTextLibrary.Conv_TextToString` _tiempodecarrera))
        (`TextBlock.SetText` (`/Game/Interfaces/BP_GUI_Carrera.TX_BESTTIME` _interface) _tiempodecarrera)
        (`KismetSystemLibrary.PrintString` (`KismetTextLibrary.Conv_TextToString` _tiempodecarrera))
        (else
          (if (not (`KismetStringLibrary.EqualEqual_StrStr` (`/Game/Interfaces/FZero_GameInstance.ModoJuego` (`self.GameInstance`)) "GP"))
            (`/Game/Interfaces/BP_GUI_Carrera.ComprobarVuelta` _interface)
            (set `self.CP_1` false)
            (set `self.CP_2` false))
          (`KismetSystemLibrary.Delay` 1.0)
          (set `self.SWEscuchar` true)
          (`KismetSystemLibrary.PrintString` "Hello")))
      (else
        (set `self.CP_1` false)
        (set `self.CP_2` false)
        (set `self.SWEscuchar` true)))))

(fn `UserConstructionScript`)